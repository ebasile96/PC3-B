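; Ship Blueprint for a player-steered ship that constantly moves forward.
; Every Tick it applies a fixed forward-vector force at the static mesh's center of mass, then adds world yaw and pitch rotation scaled by delta time.
; The Steer Ship and Up/Down axis inputs are clamp-mapped into turn rates, with yaw allowed a wider range than pitch.
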(event `self.ReceiveTick`
  (params (DeltaSeconds :type "Float (single-precision)"))
  (bind (_returnvalue_x _returnvalue_y _returnvalue_z) (`KismetMathLibrary.BreakVector` (`self.GetActorForwardVector`)))
  ;[1 1 1] Movement Logic
  (`PrimitiveComponent.AddForceAtLocation` (`self.StaticMesh`) (* (`KismetMathLibrary.MakeVector` _returnvalue_x _returnvalue_y _returnvalue_z) 6000.0) (`PrimitiveComponent.GetCenterOfMass` (`self.StaticMesh`) "None") "None")
  (`self.K2_AddActorWorldRotation` (`KismetMathLibrary.MakeRotator` 0.0 (* (`self.VerticalRotationAmount`) DeltaSeconds) (* (`self.RotationAmount`) DeltaSeconds))))

(event `InputAxis|Steer Ship`
  (params (AxisValue :type "Float (single-precision)"))
  ;[1 1 1] Inputs
  (set `self.RotationAmount` (`KismetMathLibrary.MapRangeClamped` AxisValue -1.0 1.0 -8.0 8.0)))

(event `InputAxis|Up/Down`
  (params (AxisValue :type "Float (single-precision)"))
  ;[1 1 1] Inputs
  (set `self.VerticalRotationAmount` (`KismetMathLibrary.MapRangeClamped` AxisValue -1.0 1.0 -3.0 3.0)))

(fn `UserConstructionScript`)