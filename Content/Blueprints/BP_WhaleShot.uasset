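; BP_WhaleShot is a shot actor, apparently a projectile, that damages the player's ship.
; When it overlaps an actor of exactly the Ship_Blueprint class, it subtracts a fixed amount from UITestShipHealth and destroys itself.
; The damage goes to player pawn 0 through a cast rather than to the overlapped actor.
; A component hit also destroys the shot, without dealing damage.
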(event `OnComponentHit_Event_0`
  (params (HitComponent :type "PrimitiveComponent Object Reference") (OtherActor :type "Actor Object Reference") (OtherComp :type "PrimitiveComponent Object Reference") (NormalImpulse :type "Vector Structure") (Hit :type "HitResult Structure (by ref)"))
  (`self.K2_DestroyActor`))

(event `self.ReceiveActorBeginOverlap`
  (params (OtherActor :type "Actor Object Reference"))
  (if (== (`GameplayStatics.GetObjectClass` OtherActor) "/Game/Blueprints/Ship_Blueprint.Ship_Blueprint_C")
    (bind _asship_blueprint (cast `/Game/Blueprints/Ship_Blueprint` (`GameplayStatics.GetPlayerPawn` 0)))
    (set `/Game/Blueprints/Ship_Blueprint.UITest_ShipHealth` (- (`/Game/Blueprints/Ship_Blueprint.UITest_ShipHealth` _asship_blueprint) 10.0) _asship_blueprint)
    (`self.K2_DestroyActor`)))

(fn `UserConstructionScript`)