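; Actor component that wraps its owning actor around a rectangular play area, teleporting it to the opposite edge when it crosses a boundary.
; Each tick it compares the owner's X and Y against the north, south, east and west limits, handling one edge at a time.
; The teleport keeps the other coordinates and rotation, and is bracketed by TeleportStart and TeleportDone dispatcher calls.
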(event `self.ReceiveBeginPlay`
  (set `self.OwnerActor` (`self.GetOwner`)))

(event `self.ReceiveTick`
  (params (DeltaSeconds :type "Float (single-precision)"))
  (bind _owneractor (`self.OwnerActor`))
  (bind _owneractor_2 (`self.OwnerActor`))
  (bind _owneractor_3 (`self.OwnerActor`))
  (bind _owneractor_4 (`self.OwnerActor`))
  (bind (_returnvalue_x _returnvalue_y _returnvalue_z) (`KismetMathLibrary.BreakVector` (`Actor.K2_GetActorLocation` _owneractor)))
  (bind (_returnvalue_x_2 _returnvalue_y_2 _returnvalue_z_2) (`KismetMathLibrary.BreakVector` (`Actor.K2_GetActorLocation` _owneractor_3)))
  (bind (_returnvalue_x_3 _returnvalue_y_3 _returnvalue_z_3) (`KismetMathLibrary.BreakVector` (`Actor.K2_GetActorLocation` _owneractor_4)))
  (bind (_returnvalue_x_4 _returnvalue_y_4 _returnvalue_z_4) (`KismetMathLibrary.BreakVector` (`Actor.K2_GetActorLocation` _owneractor_2)))
  (bind _x (.x (`KismetMathLibrary.MakeVector` (.x (`Actor.K2_GetActorLocation` (`self.OwnerActor`))) (.y (`Actor.K2_GetActorLocation` (`self.OwnerActor`))))))
  (bind _y (.y (`KismetMathLibrary.MakeVector` (.x (`Actor.K2_GetActorLocation` (`self.OwnerActor`))) (.y (`Actor.K2_GetActorLocation` (`self.OwnerActor`))))))
  (if (> _x (`self.LimitNorth`))
    (`self.TeleportStart`)
    (`Actor.K2_TeleportTo` _owneractor_4 (`KismetMathLibrary.MakeVector` (`self.LimitSouth`) _returnvalue_y_3 _returnvalue_z_3) (`Actor.K2_GetActorRotation` _owneractor_4))
    (`self.TeleportDone`)
    (elif (> _y (`self.LimitEast`))
      (`self.TeleportStart`)
      (`Actor.K2_TeleportTo` _owneractor_2 (`KismetMathLibrary.MakeVector` _returnvalue_x_4 (`self.LimitWeast`) _returnvalue_z_4) (`Actor.K2_GetActorRotation` _owneractor_2))
      (`self.TeleportDone`)
      (elif (< _x (`self.LimitSouth`))
        (`self.TeleportStart`)
        (`Actor.K2_TeleportTo` _owneractor_3 (`KismetMathLibrary.MakeVector` (`self.LimitNorth`) _returnvalue_y_2 _returnvalue_z_2) (`Actor.K2_GetActorRotation` _owneractor_3))
        (`self.TeleportDone`)
        (elif (< _y (`self.LimitWeast`))
          (`self.TeleportStart`)
          (`Actor.K2_TeleportTo` _owneractor (`KismetMathLibrary.MakeVector` _returnvalue_x (`self.LimitEast`) _returnvalue_z) (`Actor.K2_GetActorRotation` _owneractor))
          (`self.TeleportDone`))))))