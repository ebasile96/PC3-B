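; BP_limitMovShip is an actor component that keeps its owning ship within an altitude band.
; On BeginPlay it caches the owner as ShipRef.
; Every tick, if that reference is valid, it sets the ship's location with Z clamped between MinAltitudine and MaxAltitudine, leaving X and Y unchanged.
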(event `self.ReceiveBeginPlay`
  (set `self.ShipRef` (`self.GetOwner`)))

(event `self.ReceiveTick`
  (params (DeltaSeconds :type "Float (single-precision)"))
  (bind _shipref (`self.ShipRef`))
  (bind (_returnvalue_x _returnvalue_y _returnvalue_z) (`KismetMathLibrary.BreakVector` (`Actor.K2_GetActorLocation` _shipref)))
  (`/Engine/EditorBlueprintResources/StandardMacros.IsValid` _shipref
    (:`Is Valid`
      (`Actor.K2_SetActorLocation` (`self.ShipRef`) (`KismetMathLibrary.MakeVector` _returnvalue_x _returnvalue_y (`KismetMathLibrary.FClamp` _returnvalue_z (`self.Min Altitudine`) (`self.Max Altitudine`))) false false))))