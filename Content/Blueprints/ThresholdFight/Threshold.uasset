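; Threshold prototypes a rope-tension balancing fight, with tension starting just under a midpoint that it drifts away from.
; Tick uses Delay nodes to pace the drift, adding faster drift near either extreme and printing rewrap, unwrap and broken-threshold states.
; The Steer Ship axis nudges tension up on positive input and down otherwise, including at rest.
; Outcomes are only debug prints, and SetRTPerpetualIncrease is never called here.
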(event `self.ReceiveBeginPlay`
  (set `self.Rope Tension` 49.990002))

(event `self.ReceiveTick`
  (params (DeltaSeconds :type "Float (single-precision)"))
  (`KismetSystemLibrary.PrintString` (`KismetStringLibrary.Conv_DoubleToString` (`self.Rope Tension`)) true true (struct :`G` 0.770833 :`B` 0.145423 :`A` 1.0) (`GameplayStatics.GetWorldDeltaSeconds`))
  (if (>= (`self.Rope Tension`) 50.0)
    (`KismetSystemLibrary.Delay` 1.0)
    (set `self.Rope Tension` (+ (`self.Rope Tension`) 2.0))
    (if (>= (`self.Rope Tension`) 70.0)
      (`KismetSystemLibrary.PrintString` "ACTIVE REWRAP" true true (struct :`R` 1.0 :`B` 0.884553 :`A` 1.0))
      (if (>= (`self.Rope Tension`) 80.0)
        (`KismetSystemLibrary.Delay` 1.0)
        (set `self.Rope Tension` (+ (`self.Rope Tension`) 5.0))
        (if (>= (`self.Rope Tension`) 100.0)
          (`KismetSystemLibrary.PrintString` "Threshold Broken" true true (struct :`R` 1.0 :`B` 0.156202 :`A` 1.0)))))
    (else
      (`KismetSystemLibrary.Delay` 1.0)
      (set `self.Rope Tension` (+ (`self.Rope Tension`) -2.0))
      (if (<= (`self.Rope Tension`) 30.0)
        (`KismetSystemLibrary.PrintString` "ACTIVE UNWRAP" true true (struct :`R` 1.0 :`B` 0.884553 :`A` 1.0))
        (if (<= (`self.Rope Tension`) 20.0)
          (`KismetSystemLibrary.Delay` 1.0)
          (set `self.Rope Tension` (+ (`self.Rope Tension`) -5.0))
          (if (<= (`self.Rope Tension`) 0.0)
            (`KismetSystemLibrary.PrintString` "Threshold Broken" true true (struct :`R` 1.0 :`B` 0.156202 :`A` 1.0))))))))

(event `InputAxis|Steer Ship`
  (params (AxisValue :type "Float (single-precision)"))
  (if (> (`KismetMathLibrary.MapRangeClamped` AxisValue -1.0 1.0 -1.0 1.0) 0.001)
    (`KismetSystemLibrary.Delay` 0.2)
    (set `self.Rope Tension` (+ (`self.Rope Tension`) 1.0))
    (else
      (`KismetSystemLibrary.Delay` 0.2)
      (set `self.Rope Tension` (+ (`self.Rope Tension`) -1.0)))))

(fn `Set RT Perpetual Increase`
  (set `self.Rope Tension` (+ (`self.Rope Tension`) 2.0)))

(fn `UserConstructionScript`)