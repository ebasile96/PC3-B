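; AI whale enemy that wanders freely and attacks the player's ship.
; Each Tick a large sphere trace looks for Ship_Blueprint; on a hit it faces the ship, moves the mesh toward the impact point and fires BP_WhaleShot after a delay.
; Otherwise a random MultiGate picks movement impulses, using six directional capsule overlaps to steer away from obstacles.
; Random forward bursts and a yaw rate that can flip create circular wandering.
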(event `self.CapsuleFront.OnComponentBeginOverlap`
  (params (OverlappedComponent :type "PrimitiveComponent Object Reference") (OtherActor :type "Actor Object Reference") (OtherComp :type "PrimitiveComponent Object Reference") (OtherBodyIndex :type Integer) (bFromSweep :type Boolean) (SweepResult :type "HitResult Structure (by ref)"))
  ;[1 0.1692 0.586 1 39] Collision Detection from Capsules
  (set `self.OverlappedFRONT` true))

(event `self.CapsuleRIGHT.OnComponentBeginOverlap`
  (params (OverlappedComponent :type "PrimitiveComponent Object Reference") (OtherActor :type "Actor Object Reference") (OtherComp :type "PrimitiveComponent Object Reference") (OtherBodyIndex :type Integer) (bFromSweep :type Boolean) (SweepResult :type "HitResult Structure (by ref)"))
  ;[1 0.1692 0.586 1 39] Collision Detection from Capsules
  (set `self.OverlappedRIGHT` true))

(event `GO BACK`
  (bind _skeletalmesh (`self.SkeletalMesh`))
  ;[1 0.8615 0] These are the components that add  Forward,Up and Right force.In order to move in the opposite direction all you do is add a minus
  (`PrimitiveComponent.AddImpulse` _skeletalmesh (* (`SceneComponent.GetForwardVector` _skeletalmesh) -30.0) "None" true))

(event `GO DOWN`
  (bind _skeletalmesh (`self.SkeletalMesh`))
  ;[1 0.8615 0] These are the components that add  Forward,Up and Right force.In order to move in the opposite direction all you do is add a minus
  (`PrimitiveComponent.AddImpulse` _skeletalmesh (* (`SceneComponent.GetUpVector` _skeletalmesh) -40.0) "None" true))

(event `self.CapsuleRIGHT.OnComponentEndOverlap`
  (params (OverlappedComponent :type "PrimitiveComponent Object Reference") (OtherActor :type "Actor Object Reference") (OtherComp :type "PrimitiveComponent Object Reference") (OtherBodyIndex :type Integer))
  ;[1 0.1692 0.586 1 39] Collision Detection from Capsules
  (set `self.OverlappedRIGHT` false))

(event `self.CapsuleFront.OnComponentEndOverlap`
  (params (OverlappedComponent :type "PrimitiveComponent Object Reference") (OtherActor :type "Actor Object Reference") (OtherComp :type "PrimitiveComponent Object Reference") (OtherBodyIndex :type Integer))
  ;[1 0.1692 0.586 1 39] Collision Detection from Capsules
  (set `self.OverlappedFRONT` false))

(event `GO FORWARD`
  (bind _skeletalmesh (`self.SkeletalMesh`))
  ;[1 0.8615 0] These are the components that add  Forward,Up and Right force.In order to move in the opposite direction all you do is add a minus
  (`PrimitiveComponent.AddImpulse` _skeletalmesh (* (`SceneComponent.GetForwardVector` _skeletalmesh) 30.0) "None" true))

(event `GO UP`
  (bind _skeletalmesh (`self.SkeletalMesh`))
  ;[1 0.8615 0] These are the components that add  Forward,Up and Right force.In order to move in the opposite direction all you do is add a minus
  (`PrimitiveComponent.AddImpulse` _skeletalmesh (* (`SceneComponent.GetUpVector` _skeletalmesh) 100.0) "None" true))

(event `Const Forwarding`
  (bind _skeletalmesh (`self.SkeletalMesh`))
  ;[0.6919 1 0.0235] The AI is in constant motion. It has a constant forward force and a constant rotational force, togather the AI moves in a circular motion
  (`PrimitiveComponent.AddImpulse` _skeletalmesh (* (`SceneComponent.GetForwardVector` _skeletalmesh) (`KismetMathLibrary.RandomFloatInRange` 700.0 3000.0)) "None" true))

(event `self.CapsuleBACK.OnComponentBeginOverlap`
  (params (OverlappedComponent :type "PrimitiveComponent Object Reference") (OtherActor :type "Actor Object Reference") (OtherComp :type "PrimitiveComponent Object Reference") (OtherBodyIndex :type Integer) (bFromSweep :type Boolean) (SweepResult :type "HitResult Structure (by ref)"))
  ;[1 0.1692 0.586 1 39] Collision Detection from Capsules
  (set `self.OverlappedBACK` true))

(event `self.CapsuleTOP.OnComponentBeginOverlap`
  (params (OverlappedComponent :type "PrimitiveComponent Object Reference") (OtherActor :type "Actor Object Reference") (OtherComp :type "PrimitiveComponent Object Reference") (OtherBodyIndex :type Integer) (bFromSweep :type Boolean) (SweepResult :type "HitResult Structure (by ref)"))
  ;[1 0.1692 0.586 1 39] Collision Detection from Capsules
  (set `self.OverlappedTOP` true))

(event `GO LEFT`
  (bind _skeletalmesh (`self.SkeletalMesh`))
  ;[1 0.8615 0] These are the components that add  Forward,Up and Right force.In order to move in the opposite direction all you do is add a minus
  (`PrimitiveComponent.AddImpulse` _skeletalmesh (* (`SceneComponent.GetRightVector` _skeletalmesh) -30.0) "None" true))

(event `GO RIGHT`
  (bind _skeletalmesh (`self.SkeletalMesh`))
  ;[1 0.8615 0] These are the components that add  Forward,Up and Right force.In order to move in the opposite direction all you do is add a minus
  (`PrimitiveComponent.AddImpulse` _skeletalmesh (* (`SceneComponent.GetRightVector` _skeletalmesh) 30.0) "None" true))

(event `Const Rotation`
  (bind _skeletalmesh (`self.SkeletalMesh`))
  (bind (_returnvalue_roll _returnvalue_pitch _returnvalue_yaw) (`KismetMathLibrary.BreakRotator` (`SceneComponent.K2_GetComponentRotation` _skeletalmesh)))
  ;[0.6919 1 0.0235] The AI is in constant motion. It has a constant forward force and a constant rotational force, togather the AI moves in a circular motion
  (`SceneComponent.K2_SetWorldRotation` _skeletalmesh (`KismetMathLibrary.MakeRotator` _returnvalue_roll _returnvalue_pitch (+ _returnvalue_yaw (`self.const ratation rate`))) false false)
  ;;[1 1 1] To give the AI its randomness we delay and switch the rotation value of Z
  (`KismetSystemLibrary.Delay` 4.0)
  (`|MultiGate` true
    (:`Out 0`
      (set `self.const ratation rate` 1.5))
    (:`Out 1`
      (set `self.const ratation rate` -1.5))))

(event `self.CapsuleTOP.OnComponentEndOverlap`
  (params (OverlappedComponent :type "PrimitiveComponent Object Reference") (OtherActor :type "Actor Object Reference") (OtherComp :type "PrimitiveComponent Object Reference") (OtherBodyIndex :type Integer))
  ;[1 0.1692 0.586 1 39] Collision Detection from Capsules
  (set `self.OverlappedTOP` false))

(event `self.CapsuleBACK.OnComponentEndOverlap`
  (params (OverlappedComponent :type "PrimitiveComponent Object Reference") (OtherActor :type "Actor Object Reference") (OtherComp :type "PrimitiveComponent Object Reference") (OtherBodyIndex :type Integer))
  ;[1 0.1692 0.586 1 39] Collision Detection from Capsules
  (set `self.OverlappedBACK` false))

(event `ROTATE`
  (bind _skeletalmesh (`self.SkeletalMesh`))
  (bind (_returnvalue_roll _returnvalue_pitch _returnvalue_yaw) (`KismetMathLibrary.BreakRotator` (`SceneComponent.K2_GetComponentRotation` _skeletalmesh)))
  ;[1 0.8615 0] These are the components that add  Forward,Up and Right force.In order to move in the opposite direction all you do is add a minus
  (`SceneComponent.K2_SetWorldRotation` _skeletalmesh (`KismetMathLibrary.MakeRotator` _returnvalue_roll _returnvalue_pitch (+ _returnvalue_yaw 180.0)) false false)
  (`self.GO DOWN`))

(event `self.CapsuleLEFT.OnComponentBeginOverlap`
  (params (OverlappedComponent :type "PrimitiveComponent Object Reference") (OtherActor :type "Actor Object Reference") (OtherComp :type "PrimitiveComponent Object Reference") (OtherBodyIndex :type Integer) (bFromSweep :type Boolean) (SweepResult :type "HitResult Structure (by ref)"))
  ;[1 0.1692 0.586 1 39] Collision Detection from Capsules
  (set `self.OverlappedLEFT` true))

(event `self.CapsuleDOWN.OnComponentBeginOverlap`
  (params (OverlappedComponent :type "PrimitiveComponent Object Reference") (OtherActor :type "Actor Object Reference") (OtherComp :type "PrimitiveComponent Object Reference") (OtherBodyIndex :type Integer) (bFromSweep :type Boolean) (SweepResult :type "HitResult Structure (by ref)"))
  ;[1 0.1692 0.586 1 39] Collision Detection from Capsules
  (set `self.OverlappedDOWN` true))

(event `self.CapsuleLEFT.OnComponentEndOverlap`
  (params (OverlappedComponent :type "PrimitiveComponent Object Reference") (OtherActor :type "Actor Object Reference") (OtherComp :type "PrimitiveComponent Object Reference") (OtherBodyIndex :type Integer))
  ;[1 0.1692 0.586 1 39] Collision Detection from Capsules
  (set `self.OverlappedLEFT` false))

(event `self.CapsuleDOWN.OnComponentEndOverlap`
  (params (OverlappedComponent :type "PrimitiveComponent Object Reference") (OtherActor :type "Actor Object Reference") (OtherComp :type "PrimitiveComponent Object Reference") (OtherBodyIndex :type Integer))
  ;[1 0.1692 0.586 1 39] Collision Detection from Capsules
  (set `self.OverlappedDOWN` false))

(event `AI SEARCH`
  ;[0.1451 0 1] This part Helps the AI respond to the Capsule Collison and to move
  (`|MultiGate` true true 0
    (:`Out 0`
      (if (`self.OverlappedTOP`)
        (`self.GO DOWN`)))
    (:`Out 1`
      (if (`self.OverlappedFRONT`)
        (if (`self.OverlappedTOP`)
          (`self.ROTATE`)
          (else
            (`self.GO UP`)))
        (else
          (`self.Const Forwarding`)
          (`self.Const Rotation`))))
    (:`Out 2`
      (if (`self.OverlappedDOWN`)
        (`self.GO UP`)
        (else
          (`self.GO DOWN`))))
    (:`Out 3`
      (if (`self.OverlappedLEFT`)
        (`self.GO RIGHT`)
        (else
          (`self.GO LEFT`))))
    (:`Out 4`
      (if (`self.OverlappedRIGHT`)
        (`self.GO LEFT`)
        (else
          (`self.GO RIGHT`))))
    (:`Out 5`
      (if (`self.OverlappedBACK`)
        (`self.GO FORWARD`)))))

(event `self.ReceiveTick`
  (params (DeltaSeconds :type "Float (single-precision)"))
  (bind _returnvalue (`self.K2_GetActorLocation`))
  ;[0 1 0.9474 1 24] The Mind of the AI, Decied when to follow User and when to search for user
  (bind _outactors (`GameplayStatics.GetAllActorsOfClass` "/Script/Engine.StaticMeshActor"))
  (bind _outhit (`KismetSystemLibrary.SphereTraceSingle` _returnvalue _returnvalue 15000.0 "TraceTypeQuery2" false _outactors "ForOneFrame" true (struct :`R` 1.0 :`A` 0.995) (struct :`G` 1.0 :`A` 1.0) 0.1))
  (bind (_bblockinghit _binitialoverlap _time _distance _location _impactpoint _normal _impactnormal _physmat _hitactor) (`GameplayStatics.BreakHitResult` _outhit))
  (if (`KismetStringLibrary.EqualEqual_StrStr` (`KismetSystemLibrary.GetDisplayName` _hitactor) "Ship_Blueprint")
    (bind _asship_blueprint (cast `/Game/Blueprints/Ship_Blueprint` _hitactor))
    (`self.K2_SetActorRotation` (`KismetMathLibrary.FindLookAtRotation` (`self.K2_GetActorLocation`) (`self.K2_GetActorLocation` _asship_blueprint)))
    (`self.Fire Shot`)
    (`KismetSystemLibrary.MoveComponentTo` (`self.SkeletalMesh`) (`KismetMathLibrary.MakeVector` (.x (- _impactpoint (150.0 150.0 0.0))) (.y (- _impactpoint (150.0 150.0 0.0))) (+ (.z (- _impactpoint (150.0 150.0 0.0))) 30.0)) (struct) true true 2.5)
    (else
      (`self.AI SEARCH`))))

(event `Fire Shot`
  (bind _arrow (`self.Arrow`))
  ;[1 1 1] Firing Shots
  (`KismetSystemLibrary.Delay` 2.0)
  (`|SpawnActorFromClass` "/Game/Blueprints/BP_WhaleShot.BP_WhaleShot_C" (`KismetMathLibrary.MakeTransform` (`SceneComponent.K2_GetComponentLocation` _arrow) (`KismetMathLibrary.Conv_VectorToRotator` (`SceneComponent.GetForwardVector` _arrow))) "AlwaysSpawn" "OverrideRootScale" null null))

(fn `UserConstructionScript`)