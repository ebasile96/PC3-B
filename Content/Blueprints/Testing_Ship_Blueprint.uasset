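; Test player ship pawn that moves constantly forward with gear-based speed, steering and pitch, tilting its mesh by interpolation.
; Timelines move the spring-arm camera between panoramic, cannon-aim and harpoon views.
; A camera line trace sets the target for angle-limited cannon broadsides, chosen by look direction and reload-delayed, and for harpoon shots.
; Tick also checks distance to a "Whale"-tagged actor; debug inputs toggle test UI and reduce health.
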(event `self.ReceiveBeginPlay`
  (`|ExecutionSequence`
    (:`then_0`
      (bind _returnvalue (`|CreateWidget` "/Game/Blueprints/BP_Controls.BP_Controls_C"))
      (`UserWidget.AddToViewport` _returnvalue 0))
    (:`then_1`
      (`CableComponent.SetAttachEndToComponent` (`self.Rope`) (`self.HarpoonProjectile`) "RopeAttachment"))))

(event `self.ReceiveTick`
  (params (DeltaSeconds :type "Float (single-precision)"))
  (bind _returnvalue (`self.GetInputAxisValue`))
  (bind _returnvalue_2 (`self.GetInputAxisValue`))
  ;[1 1 1] tick
  (`|ExecutionSequence`
    (:`then_0`
      (`PawnMovementComponent.AddInputVector` (`self.FloatingPawnMovement`) (`self.GetActorForwardVector`) false)
      (`self.K2_AddActorWorldRotation` (`KismetMathLibrary.MakeRotator` 0.0 0.0 (* (`self.RotationAmount`) DeltaSeconds)))
      (`self.K2_AddActorLocalRotation` (`KismetMathLibrary.MakeRotator` 0.0 (* (`self.VerticalRotationAmount`) DeltaSeconds))))
    (:`then_1`
      (bind _returnvalue_3 (`self.LookingDirection`))
      (if (> _returnvalue_3 0.0)
        (bind _returnvalue_4 (`self.SetCannonsToShoot` (`self.CannonsRight`)))
        (set `self.CannonsToSHoot` _returnvalue_4)
        (else
          (bind _returnvalue_5 (`self.SetCannonsToShoot` (`self.CannonsLeft`)))
          (set `self.CannonsToSHoot` _returnvalue_5))))
    (:`then_2`
      (if (== _returnvalue_2 0.0)
        (set `self.targetVerticalRoll` 0.0)
        (elif (> _returnvalue_2 0.0)
          (set `self.targetVerticalRoll` 10.0)
          (else
            (set `self.targetVerticalRoll` -10.0))))
      (set `self.actualVerticalRoll` (`KismetMathLibrary.FInterpTo` (`self.actualVerticalRoll`) (`self.targetVerticalRoll`) (`GameplayStatics.GetWorldDeltaSeconds`) 2.0))
      (if (== _returnvalue 0.0)
        (set `self.TargetRoll` 0.0)
        (elif (> _returnvalue 0.0)
          (set `self.TargetRoll` 10.0)
          (else
            (set `self.TargetRoll` -10.0))))
      (set `self.ActualRoll` (`KismetMathLibrary.FInterpTo` (`self.ActualRoll`) (`self.TargetRoll`) (`GameplayStatics.GetWorldDeltaSeconds`) 2.0))
      (`SceneComponent.K2_SetRelativeRotation` (`self.StaticMeshComponent`) (`KismetMathLibrary.MakeRotator` (`self.ActualRoll`) (`self.actualVerticalRoll`)) false false))
    (:`then_3`
      (`self.CameraLookSetter`))
    (:`then_4`
      (if (`self.HurlMode`)
        (`SceneComponent.K2_SetWorldRotation` (`self.HarpoonCannon`) (`SceneComponent.K2_GetComponentRotation` (`self.CameraComponent`)) false false)))
    (:`then_5`
      (bind _distance (`self.GetWhaleDistance`))
      (bind _output_get (set `self.DistanceFromWhale` _distance))
      (if (> _output_get (`self.ThresholdDistanceValue`))
        (set `self.Threshold distance` false)
        (`KismetSystemLibrary.PrintString` "off distance" true true (struct :`R` 1.0 :`B` 0.02989 :`A` 1.0))
        (else
          (set `self.Threshold distance` true)
          (`KismetSystemLibrary.PrintString` "in distance" true true (struct :`R` 0.039156 :`G` 1.0 :`A` 1.0)))))))

(event `InputAxis|Steer Ship`
  (params (AxisValue :type "Float (single-precision)"))
  ;[1 1 1] Inputs
  (set `self.RotationAmount` (`KismetMathLibrary.MapRangeClamped` AxisValue -1.0 1.0 -8.0 8.0)))

(event `InputAction|GearUp`
  (params (Key :type "Key Structure"))
  ;[1 1 1] Inputs
  (:`Pressed`
    (bind _returnvalue (`self.ShiftGearUp`))
    (bind _output_get (set `self.CurrentGearValue` _returnvalue))
    (set `FloatingPawnMovement.MaxSpeed` (* _output_get 1.0) (`self.FloatingPawnMovement`))
    (`KismetSystemLibrary.PrintString` (`self.CurrentGearName`))))

(event `InputAction|Fire`
  (params (Key :type "Key Structure"))
  ;[1 1 1] Inputs
  (:`Pressed`
    (if (`self.Reloading`)
      _
      (elif (`self.Aiming`)
        (`self.CannonFire`)
        (set `self.Reloading` true)
        (`|ExecutionSequence`
          (:`then_0`
            (`KismetSystemLibrary.Delay` 2.0)
            (`|ExecutionSequence`
              (:`then_0`
                (set `self.Reloading` false))
              (:`then_1`
                (`KismetSystemLibrary.PrintString` "ready to shoot!"))))
          (:`then_1`
            (`KismetSystemLibrary.PrintString` "reloading")))))))

(event `InputAction|GearDown`
  (params (Key :type "Key Structure"))
  ;[1 1 1] Inputs
  (:`Pressed`
    (bind _returnvalue (`self.ShiftGearDown`))
    (bind _output_get (set `self.CurrentGearValue` _returnvalue))
    (set `FloatingPawnMovement.MaxSpeed` (* _output_get 1.0) (`self.FloatingPawnMovement`))
    (`KismetSystemLibrary.PrintString` (`self.CurrentGearName`))))

(event `InputAxis|Up/Down`
  (params (AxisValue :type "Float (single-precision)"))
  ;[1 1 1] Inputs
  (set `self.VerticalRotationAmount` (`KismetMathLibrary.MapRangeClamped` AxisValue -1.0 1.0 -3.0 3.0)))

(event `InputAction|Fire`
  (params (Key :type "Key Structure"))
  (bind _returnvalue (`SceneComponent.GetSocketLocation` (`self.HarpoonCannon`) "FireHarpoon"))
  ;[1 1 1] harpoon projectile
  (:`Pressed`
    (if (`self.HurlMode`)
      (bind _angle (`self.CalculateFireAngle` (`SceneComponent.GetForwardVector` (`self.CameraComponent`)) (`SceneComponent.GetForwardVector` (`self.HarpoonCannon`))))
      (if (`KismetMathLibrary.InRange_FloatFloat` _angle -30.0 30.0)
        (`|SpawnActorFromClass` "/Game/Blueprints/BP_HarpoonProjectile.BP_HarpoonProjectile_C" (`KismetMathLibrary.MakeTransform` _returnvalue (`KismetMathLibrary.FindLookAtRotation` _returnvalue (`self.CameraLook`))) "AlwaysSpawn" "OverrideRootScale" null null)
        (`GameplayStatics.SpawnSoundAtLocation` "/Game/SoundFX/Harpoon/SFX_HarpoonShot.SFX_HarpoonShot" _returnvalue (struct) 1.0 1.0 0.0 null null)))))

(event `InputAxis|CameraMovX`
  (params (AxisValue :type "Float (single-precision)"))
  ;[1 1 1] Camera
  (`self.AddControllerYawInput` AxisValue))

(event `InputAxis|CameraMovY`
  (params (AxisValue :type "Float (single-precision)"))
  ;[1 1 1] Camera
  (`self.AddControllerPitchInput` AxisValue))

(event `InputAction|GoToPanoramicCamera`
  (params (Key :type "Key Structure"))
  ;[1 1 1] Panoramic Camera
  (:`Pressed`
    (set `self.PanoramicMode` true)
    (bind (_direction _springlength) (`Timeline|PanoramicCameraTimeLIne`)
      (:`Update`
        (`|ExecutionSequence`
          (:`then_0`
            (set `SpringArmComponent.TargetArmLength` _springlength (`self.SpringArmComponent`))))))))

(event `InputAction|CannonAim`
  (params (Key :type "Key Structure"))
  ;[1 1 1] Cannon Camera
  (:`Pressed`
    (set `self.currentCamLocation` (`SceneComponent.RelativeLocation` (`self.SpringArmComponent`)))
    (bind (_direction _alpha _arm_length) (`Timeline|cannonCamera` :!label _label)
      (:`Update`
        (`|ExecutionSequence`
          (:`then_0`
            (`SceneComponent.K2_SetRelativeLocation` (`self.SpringArmComponent`) (`KismetMathLibrary.VLerp` (`self.currentCamLocation`) (`SceneComponent.RelativeLocation` (`self.CannonCameraLocation`)) _alpha) false false)
            (set `SpringArmComponent.TargetArmLength` _arm_length (`self.SpringArmComponent`)))
          (:`then_1`
            (switch `ETimelineDirection` _direction
              (:`Forward`
                (set `self.Aiming` true))
              (:`Backward`
                (set `SpringArmComponent.TargetArmLength` 562.0 (`self.SpringArmComponent`))
                (set `self.Aiming` false))))
          (:`then_2`
            (switch `ETimelineDirection` _direction
              (:`Forward`
                (bind _returnvalue (`|CreateWidget` "/Game/Blueprints/BP_Crosshair.BP_Crosshair_C"))
                (bind _output_get (set `self.CrossairHUD` _returnvalue))
                (`UserWidget.AddToViewport` _output_get 0))
              (:`Backward`
                (`|ExecutionSequence`
                  (:`then_0`
                    (`Widget.RemoveFromParent` _output_get))))))))))
  (:`Released`
    (goto _label :!via `Reverse`)))

(event `InputAction|GoToPanoramicCamera`
  (params (Key :type "Key Structure"))
  ;[1 1 1] Panoramic Camera
  (:`Pressed`
    (if (`self.PanoramicMode`)
      (bind (_direction _springlength) (`Timeline|PanoramicCamera2`)
        (:`Update`
          (`|ExecutionSequence`
            (:`then_0`
              (set `SpringArmComponent.TargetArmLength` _springlength (`self.SpringArmComponent`)))))
        (:`Finished`
          (set `self.PanoramicMode` false))))))

(event `InputAction|GoToHurlCamera`
  (params (Key :type "Key Structure"))
  ;[1 1 1] Harpoon camera
  (:`Pressed`
    (set `self.HurlMode` true)
    (set `self.currentCamLocation` (`SceneComponent.RelativeLocation` (`self.SpringArmComponent`)))
    (bind (_direction _alpha _arm_length) (`Timeline|Timeline_0`)
      (:`Update`
        (`|ExecutionSequence`
          (:`then_0`
            (`SceneComponent.K2_SetRelativeLocation` (`self.SpringArmComponent`) (`KismetMathLibrary.VLerp` (`self.currentCamLocation`) (`SceneComponent.RelativeLocation` (`self.HarpoonCameraLocation`)) _alpha) false false)
            (set `SpringArmComponent.TargetArmLength` _arm_length (`self.SpringArmComponent`)))
          (:`then_1`
            (switch `ETimelineDirection` _direction
              (:`Forward`
                (bind _returnvalue (`|CreateWidget` "/Game/Blueprints/BP_Crosshair.BP_Crosshair_C"))
                (bind _output_get (set `self.CrossairHUD` _returnvalue))
                (`UserWidget.AddToViewport` _output_get 0)))))))))

(event `InputAction|GoToHurlCamera`
  (params (Key :type "Key Structure"))
  ;[1 1 1] Harpoon camera
  (:`Pressed`
    (if (`self.HurlMode`)
      (set `self.currentCamLocation` (`SceneComponent.RelativeLocation` (`self.SpringArmComponent`)))
      (bind (_direction _alpha _arm_length) (`Timeline|Timeline_1`)
        (:`Update`
          (`|ExecutionSequence`
            (:`then_0`
              (`SceneComponent.K2_SetRelativeLocation` (`self.SpringArmComponent`) (`KismetMathLibrary.VLerp` (`self.currentCamLocation`) (`SceneComponent.RelativeLocation` (`self.HelmCameraLocation`)) _alpha) false false)
              (set `SpringArmComponent.TargetArmLength` _arm_length (`self.SpringArmComponent`)))
            (:`then_1`
              (switch `ETimelineDirection` _direction
                (:`Backward`
                  (`|ExecutionSequence`
                    (:`then_0`
                      (`Widget.RemoveFromParent` (`self.CrossairHUD`)))))))))
        (:`Finished`
          (set `self.HurlMode` false))))))

(event `InputAction|ToggleUI`
  (params (Key :type "Key Structure"))
  ;[1 1 1] UI Toggle
  (:`Pressed`
    (`/Engine/EditorBlueprintResources/StandardMacros.FlipFlop`
      (:`A`
        (bind _returnvalue (`|CreateWidget` "/Game/Blueprints/BP_UITest.BP_UITest_C"))
        (bind _output_get (set `self.UI TEST` _returnvalue))
        (`UserWidget.AddToViewport` _output_get 0))
      (:`B`
        (`Widget.RemoveFromParent` (`self.UI TEST`))))))

(event `InputAction|-10 HP ShipHealth`
  (params (Key :type "Key Structure"))
  (:`Pressed`
    (set `self.UITest_ShipHealth` (- (`self.UITest_ShipHealth`) 10.0))))

(fn `CalculateFireAngle`
  (params (`Vector A` :type "Vector Structure") (`Vector B` :type "Vector Structure"))
  (returns (Angle :type "Float (double-precision)"))
  (return (`KismetMathLibrary.DegAcos` (`KismetMathLibrary.Dot_VectorVector` (`KismetMathLibrary.Normal` `Vector A` 0.0) (`KismetMathLibrary.Normal` `Vector B` 0.0)))))

(fn `CameraLookSetter`
  (bind _returnvalue (`SceneComponent.K2_GetComponentLocation` (`self.CameraComponent`)))
  (bind (_outhit _returnvalue_2) (`KismetSystemLibrary.LineTraceSingle` _returnvalue (+ (* (`SceneComponent.GetForwardVector` (`self.CameraComponent`)) (`self.RayLength`)) _returnvalue) "TraceTypeQuery1"))
  (bind (_bblockinghit _binitialoverlap _time _distance _location _impactpoint _normal _impactnormal _physmat _hitactor _hitcomponent _hitbonename _hititem _faceindex _tracestart _traceend) (`GameplayStatics.BreakHitResult` _outhit))
  (set `self.CameraLook` (`KismetMathLibrary.SelectVector` _impactpoint _traceend _returnvalue_2)))

(fn `CannonFire`
  (bind _returnvalue (`KismetMathLibrary.FindLookAtRotation` (`SceneComponent.K2_GetComponentLocation` (`|GetArrayItem` (`self.CannonsToSHoot`) 1)) (`self.CameraLook`)))
  (bind _angle (`self.CalculateFireAngle` (`self.GetActorForwardVector`) (`SceneComponent.GetForwardVector` (`self.CameraComponent`))))
  (if (`KismetMathLibrary.InRange_FloatFloat` _angle 50.0 140.0)
    (`SceneComponent.K2_SetWorldRotation` (`|GetArrayItem` (`self.CannonsToSHoot`) 1) _returnvalue false false)
    (for _array_element (`self.CannonsToSHoot`)
      (`SceneComponent.K2_SetWorldRotation` _array_element _returnvalue false false))
    (for _array_element_2 (`self.CannonsToSHoot`)
      (bind _returnvalue_2 (`SceneComponent.K2_GetComponentLocation` _array_element_2))
      (bind _returnvalue_3 (`SceneComponent.K2_GetComponentRotation` _array_element_2))
      (`|SpawnActorFromClass` "/Game/Blueprints/BP_CannonBall.BP_CannonBall_C" (`KismetMathLibrary.MakeTransform` _returnvalue_2 _returnvalue_3) "Undefined" "OverrideRootScale" null null)
      (`NiagaraFunctionLibrary.SpawnSystemAtLocation` "/Game/VFX/Cannons/CannonExplosion.CannonExplosion" _returnvalue_2 _returnvalue_3 (0.8 0.8 0.8))
      (`GameplayStatics.SpawnSoundAtLocation` "/Game/SoundFX/Cannon/SFX_CannonFire.SFX_CannonFire" _returnvalue_2 (struct) 1.0 1.0 0.0 null null))))

(fn `GetWhaleDistance`
  (returns (Distance :type "Float (double-precision)"))
  (bind _outactors (`GameplayStatics.GetAllActorsOfClassWithTag` "/Script/Engine.Actor" "Whale"))
  (for _array_element _outactors
    (return (`KismetMathLibrary.Vector_Distance` (`self.K2_GetActorLocation`) (`self.K2_GetActorLocation` _array_element)))))

(fn `InstanciateAimingSpline`
  (for _array_element (`self.CannonsToSHoot`)
    (bind _returnvalue (`SceneComponent.K2_GetComponentLocation` _array_element))
    (bind _returnvalue_2 (`|SpawnActorFromClass` "/Game/Blueprints/BP_AimSpline.BP_AimSpline_C" (`KismetMathLibrary.MakeTransform` _returnvalue (`KismetMathLibrary.FindLookAtRotation` _returnvalue (`self.CameraLook`))) "Undefined" "OverrideRootScale" null null))
    (set `self.SplineInstance` _returnvalue_2)))

(fn `LockCamera`
  (bind _returnvalue (`GameplayStatics.GetPlayerCameraManager` 0))
  (bind _returnvalue_2 (`GameplayStatics.GetPlayerCameraManager` 0))
  (bind _returnvalue_3 (`GameplayStatics.GetPlayerCameraManager` 0))
  (if (`self.Aiming`)
    (bind _returnvalue_4 (`self.LookingDirection`))
    (if (> _returnvalue_4 0.0)
      (set `PlayerCameraManager.ViewYawMin` 0.0 _returnvalue_2)
      (set `PlayerCameraManager.ViewYawMax` 180.0 _returnvalue_2)
      (else
        (set `PlayerCameraManager.ViewYawMin` 180.0 _returnvalue_3)
        (set `PlayerCameraManager.ViewYawMax` 359.98999 _returnvalue_3)))
    (else
      (set `PlayerCameraManager.ViewYawMin` 0.0 _returnvalue)
      (set `PlayerCameraManager.ViewYawMax` 359.98999 _returnvalue))))

(fn `UserConstructionScript`
  (`CableComponent.SetAttachEndToComponent` (`self.Rope`) (`self.HarpoonProjectile`) "RopeAttachment"))