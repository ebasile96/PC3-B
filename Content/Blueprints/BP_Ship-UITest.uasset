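; BP_Ship-UITest is a player-controlled ship pawn with a toggleable test UI and a debug input that lowers ship health.
; Tick constantly drives the FloatingPawnMovement forward, with gear shifts setting max speed and axis inputs setting yaw and pitch rates.
; Steering also banks the mesh through interpolated roll.
; Cannon aim zooms the FOV by timeline and calls LockAim; distance-based crosshair logic is disconnected.
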(event `InputAction|ToggleUI`
  (params (Key :type "Key Structure"))
  ;[1 1 1] UI Toggle
  (:`Pressed`
    (`/Engine/EditorBlueprintResources/StandardMacros.FlipFlop`
      (:`A`
        (bind _returnvalue (`|CreateWidget` "/Game/Blueprints/BP_UITest.BP_UITest_C"))
        (set `self.UITest` _returnvalue)
        (`UserWidget.AddToViewport` _returnvalue 0))
      (:`B`
        (`Widget.RemoveFromParent` (`self.UITest`))))))

(event `self.ReceiveTick`
  (params (DeltaSeconds :type "Float (single-precision)"))
  ;[1 1 1] tick
  (`self.CheckTargetDistance`)
  (`PawnMovementComponent.AddInputVector` (`self.FloatingPawnMovement`) (`self.GetActorForwardVector`) false)
  (`self.K2_AddActorWorldRotation` (`KismetMathLibrary.MakeRotator` 0.0 (* (`self.VerticalRotationAmount`) DeltaSeconds) (* (`self.RotationAmount`) DeltaSeconds))))

(event `InputAction|-10 HP ShipHealth`
  (params (Key :type "Key Structure"))
  (:`Pressed`
    (set `self.UITest_ShipHealth` (- (`self.UITest_ShipHealth`) 10.0))))

(event `InputAxis|Steer Ship`
  (params (AxisValue :type "Float (single-precision)"))
  ;[1 1 1] Inputs
  (set `self.RotationAmount` (`KismetMathLibrary.MapRangeClamped` AxisValue -1.0 1.0 -8.0 8.0)))

(event `InputAction|GearUp`
  (params (Key :type "Key Structure"))
  ;[1 1 1] Inputs
  (:`Pressed`
    (bind _returnvalue (`self.ShiftGearUp`))
    (bind _output_get (set `self.CurrentGearValue` _returnvalue))
    (set `FloatingPawnMovement.MaxSpeed` (* _output_get 60.0) (`self.FloatingPawnMovement`))))

(event `InputAction|GearDown`
  (params (Key :type "Key Structure"))
  ;[1 1 1] Inputs
  (:`Pressed`
    (bind _returnvalue (`self.ShiftGearDown`))
    (bind _output_get (set `self.CurrentGearValue` _returnvalue))
    (set `FloatingPawnMovement.MaxSpeed` (* _output_get 60.0) (`self.FloatingPawnMovement`))))

(event `InputAxis|Up/Down`
  (params (AxisValue :type "Float (single-precision)"))
  ;[1 1 1] Inputs
  (set `self.VerticalRotationAmount` (`KismetMathLibrary.MapRangeClamped` AxisValue -1.0 1.0 -3.0 3.0)))

(event `InputAxis|Steer Ship`
  (params (AxisValue :type "Float (single-precision)"))
  (bind _returnvalue (`self.GetInputAxisValue`))
  ;[1 1 1] SHIP ROLL
  (if (== _returnvalue 0.0)
    (set `self.TargetRoll` 0.0)
    (elif (> _returnvalue 0.0)
      (set `self.TargetRoll` 10.0)
      (else
        (set `self.TargetRoll` -10.0))))
  (set `self.ActualRoll` (`KismetMathLibrary.FInterpTo` (`self.ActualRoll`) (`self.TargetRoll`) (`GameplayStatics.GetWorldDeltaSeconds`) 2.0))
  (`SceneComponent.K2_SetRelativeRotation` (`self.StaticMeshComponent`) (`KismetMathLibrary.MakeRotator` (`self.ActualRoll`)) false false))

(event `InputAxis|CameraMovX`
  (params (AxisValue :type "Float (single-precision)"))
  ;[1 1 1] Camera
  (`self.AddControllerYawInput` AxisValue))

(event `InputAction|CannonAim`
  (params (Key :type "Key Structure"))
  ;[1 1 1] Camera
  (:`Pressed`
    (`|ExecutionSequence`
      (:`then_0`
        (bind (_direction _alpha) (`Timeline|Camera Zoom` :!label _label)
          (:`Update`
            (`|ExecutionSequence`
              (:`then_0`
                (`CameraComponent.SetFieldOfView` (`self.CameraComponent`) (`KismetMathLibrary.Lerp` 90.0 50.0 _alpha)))
              (:`then_1`
                (`self.LockAim`))))))))
  (:`Released`
    (`|ExecutionSequence`
      (:`then_0`
        (goto _label :!via `Reverse`)))))

(event `InputAxis|CameraMovY`
  (params (AxisValue :type "Float (single-precision)"))
  ;[1 1 1] Camera
  (`self.AddControllerPitchInput` AxisValue))

(fn `UserConstructionScript`)